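; Infantry unit Blueprint (步兵03) that layers a material-driven damage effect, apparently a death dissolve, onto its parent class.
; On BeginPlay it applies one dynamic instance of M_DeadMaterial_Inst to every material slot of the 步兵待机 (infantry idle) component.
; CSIFMakeDamage calls the parent, reveals that component and plays a timeline that drives the "power" parameter and hides the main Mesh on an event track.
; CSIFFly only forwards to the parent, and AttackCS is empty.
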(event EventBeginPlay
  (bind _步兵待机 (Variables|Default|Get步兵待机))
  (|CallParentFunction)
  (bind _returnvalue (Rendering|Material|CreateDynamicMaterialInstance "/Game/15/Materials/死亡/M_DeadMaterial_Inst.M_DeadMaterial_Inst" "None" "None" :!class /Script/Engine.KismetMaterialLibrary))
  (Variables|Default|SetDy _returnvalue)
  (for _index (range 0 (- (Rendering|Material|GetNumMaterials _步兵待机) 1))
    (Rendering|Material|SetMaterial _步兵待机 _index (Variables|Default|GetDy))))

(event Collision|EventActorBeginOverlap
  (params (OtherActor :type Actor%20Object%20Reference)))

(event EventTick
  (params (DeltaSeconds :type Float%20%28single-precision%29))
  (|CallParentFunction DeltaSeconds) ; 此节点被禁用，将不会被调用。\n从引脚连出引线来编译功能。
)

(event EventCSIFMakeDamage
  (params (Damage :type Float%20%28single-precision%29))
  (|CallParentFunction Damage)
  (Rendering|SetVisibility (Variables|Default|Get步兵待机) true false)
  (bind _新建轨道_0 (Timeline|时间轴_0 PlayFromStart)
    (:Update
      (Rendering|Material|SetScalarParameterValue (Variables|Default|GetDy) "power" (* _新建轨道_0 1.0) :!class /Script/Engine.MaterialInstanceDynamic))
    (:新建轨道_1
      (Rendering|SetVisibility (Variables|Character|GetMesh) false false))))

(event EventAttackCS)

(event EventCSIFFly
  (params (Point :type Vector :default "0, 0, 0") (Speed :type Vector :default "0, 0, 0"))
  (|CallParentFunction Point Speed))

(fn ConstructionScript
  (|CallParentFunction))