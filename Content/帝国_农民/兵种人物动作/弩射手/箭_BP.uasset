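; Arrow projectile for the crossbowman that flies a ballistic arc to a target landing point.
; The construction script solves launch velocity from landing point, flight time and custom gravity, rescaling projectile gravity to match.
; Overlapping a non-instigator of another faction, checked by interface message, attaches it to the hit bone, sends fixed heavy damage, then destroys it next tick.
; When projectile movement stops, effects and collision switch off before delayed destruction.
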(event OnProjectileStop(ProjectileMovement)
  (params (ImpactResult :type Hit%20Result%20Structure%20%28by%20ref%29))
  (Components|Activation|SetActive (Variables|Default|GetParticleSystem1) false true)
  (Collision|SetActorEnableCollision false)
  (Utilities|FlowControl|Delay 2.0)
  (Actor|DestroyActor))

(event OnComponentBeginOverlap(Sphere1)
  (params (OverlappedComponent :type Primitive%20Component%20Object%20Reference) (OtherActor :type Actor%20Object%20Reference) (OtherComp :type Primitive%20Component%20Object%20Reference) (OtherBodyIndex :type Integer) (bFromSweep :type Boolean) (SweepResult :type Hit%20Result%20Structure%20%28by%20ref%29))
  (if (!= OtherActor (Game|GetInstigator))
    (bind _ai (Class|CSIFAI|CSIFGet阵营(Message) OtherActor))
    (if (Utilities|Enum|NotEqual(Enum) _ai (Variables|Default|GetEnum_阵营))
      (Transformation|AttachComponentToComponent self OtherComp (.HitBoneName (Collision|BreakHitResult SweepResult)) "KeepWorld" "KeepWorld" "KeepWorld" true)
      (Components|Activation|SetActive (Variables|Default|GetParticleSystem1) false true)
      (Components|Activation|SetActive (Variables|Default|GetProjectileMovement) false true)
      (Class|CSIFAI|CSIFMakeDamage(Message) OtherActor 999.0)
      (Collision|SetActorEnableCollision false)
      (Utilities|FlowControl|Delay 0.0)
      (Actor|DestroyActor))))

(event EventBeginPlay)

(fn ConstructionScript
  (bind _projectilemovement (Variables|Default|GetProjectileMovement))
  (Variables|Default|Set初始位置 (Transformation|GetActorLocation))
  (Variables|/Script/Engine.ProjectileMovementComponent|SetProjectileGravityScale _projectilemovement (/ (Variables|Default|Get重力影响) (Components|Movement|GetGravityZ _projectilemovement)))
  (Variables|/Script/Engine.MovementComponent|SetVelocity _projectilemovement (* (Math|Vector|MakeVector (* (Math|Trig|Cos(Degrees) (.Yaw (Math|Vector|GetYawPitchfromVector (- (Variables|Default|Get落点位置) (Variables|Default|Get初始位置))))) (/ (Math|Float|Sqrt (+ (Math|Float|Square (.X (Math|Vector|BreakVector (- (Variables|Default|Get落点位置) (Variables|Default|Get初始位置))))) (Math|Float|Square (.Y (Math|Vector|BreakVector (- (Variables|Default|Get落点位置) (Variables|Default|Get初始位置))))))) (Variables|Default|Get落地时间))) (* (Math|Trig|Sin(Degrees) (.Yaw (Math|Vector|GetYawPitchfromVector (- (Variables|Default|Get落点位置) (Variables|Default|Get初始位置))))) (/ (Math|Float|Sqrt (+ (Math|Float|Square (.X (Math|Vector|BreakVector (- (Variables|Default|Get落点位置) (Variables|Default|Get初始位置))))) (Math|Float|Square (.Y (Math|Vector|BreakVector (- (Variables|Default|Get落点位置) (Variables|Default|Get初始位置))))))) (Variables|Default|Get落地时间))) (- (/ (.Z (Math|Vector|BreakVector (- (Variables|Default|Get落点位置) (Variables|Default|Get初始位置)))) (Variables|Default|Get落地时间)) (/ (* (Variables|Default|Get重力影响) (Variables|Default|Get落地时间)) 2.0))) 1.0))
  (Variables|/Script/Engine.ProjectileMovementComponent|SetInitialSpeed _projectilemovement (Math|Vector|VectorLength (Math|Vector|MakeVector (* (Math|Trig|Cos(Degrees) (.Yaw (Math|Vector|GetYawPitchfromVector (- (Variables|Default|Get落点位置) (Variables|Default|Get初始位置))))) (/ (Math|Float|Sqrt (+ (Math|Float|Square (.X (Math|Vector|BreakVector (- (Variables|Default|Get落点位置) (Variables|Default|Get初始位置))))) (Math|Float|Square (.Y (Math|Vector|BreakVector (- (Variables|Default|Get落点位置) (Variables|Default|Get初始位置))))))) (Variables|Default|Get落地时间))) (* (Math|Trig|Sin(Degrees) (.Yaw (Math|Vector|GetYawPitchfromVector (- (Variables|Default|Get落点位置) (Variables|Default|Get初始位置))))) (/ (Math|Float|Sqrt (+ (Math|Float|Square (.X (Math|Vector|BreakVector (- (Variables|Default|Get落点位置) (Variables|Default|Get初始位置))))) (Math|Float|Square (.Y (Math|Vector|BreakVector (- (Variables|Default|Get落点位置) (Variables|Default|Get初始位置))))))) (Variables|Default|Get落地时间))) (- (/ (.Z (Math|Vector|BreakVector (- (Variables|Default|Get落点位置) (Variables|Default|Get初始位置)))) (Variables|Default|Get落地时间)) (/ (* (Variables|Default|Get重力影响) (Variables|Default|Get落地时间)) 2.0))))))