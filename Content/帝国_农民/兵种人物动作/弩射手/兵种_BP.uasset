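; Crossbowman troop character with a faction and a health bar that turns toward the camera.
; It moves by spline timeline, AI MoveTo or random navmesh wandering, chosen through a movement-type enum.
; Chase and attack spheres pick enemy-faction targets and set the attack state, and attacks spawn arrow volleys with distance-scaled random scatter.
; Lethal damage stops it for delayed destruction, while knockback launches it into ragdoll before removal.
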(event OnComponentBeginOverlap(追击Sphere)
  (params (OverlappedComponent :type Primitive%20Component%20Object%20Reference) (OtherActor :type Actor%20Object%20Reference) (OtherComp :type Primitive%20Component%20Object%20Reference) (OtherBodyIndex :type Integer) (bFromSweep :type Boolean) (SweepResult :type Hit%20Result%20Structure%20%28by%20ref%29))
  ;[1 1 1] 追击范围
  (bind _as兵种_bp (Utilities|Casting|CastTo兵种_BP OtherActor))
  (if (and (!= self _as兵种_bp) (!= (Variables|兵种_BP_C|GetEnum_阵营 _as兵种_bp) (Variables|兵种属性|GetEnum_阵营)))
    (Utilities|Array|AddUnique (Variables|Default|Get目标_All) _as兵种_bp)
    (EventDispatchers|BindEventtoDestroyDis _as兵种_bp (delegate Custom|自定义事件_0))
    (Utilities|IsValid (Variables|Default|Get目标)
      (:Is%20Valid
        (if (Variables|兵种_BP_C|GetDie (Variables|Default|Get目标))
          (Variables|Default|Set目标 _as兵种_bp :!label _label)))
      (:Is%20Not%20Valid
        (goto _label)))))

(event OnComponentEndOverlap(追击Sphere)
  (params (OverlappedComponent :type Primitive%20Component%20Object%20Reference) (OtherActor :type Actor%20Object%20Reference) (OtherComp :type Primitive%20Component%20Object%20Reference) (OtherBodyIndex :type Integer))
  (bind _目标_all (Variables|Default|Get目标_All))
  ;[1 1 1] 追击范围内死亡
  (bind _as兵种_bp (Utilities|Casting|CastTo兵种_BP OtherActor))
  (Utilities|Array|RemoveItem (Variables|Default|Get目标_All) _as兵种_bp)
  (Variables|Default|SetAttack false)
  (if (> (Utilities|Array|Length _目标_all) 0)
    (Variables|Default|Set目标 (Utilities|Array|Get(acopy) _目标_all))
    (CallFunction|LockRotationCF)
    (else
      (Variables|Default|Set目标 0)))
  (Variables|/Script/Engine.CharacterMovementComponent|SetMaxWalkSpeed (Variables|Character|GetCharacterMovement) 6e+02))

(event OnComponentBeginOverlap(攻击Sphere)
  (params (OverlappedComponent :type Primitive%20Component%20Object%20Reference) (OtherActor :type Actor%20Object%20Reference) (OtherComp :type Primitive%20Component%20Object%20Reference) (OtherBodyIndex :type Integer) (bFromSweep :type Boolean) (SweepResult :type Hit%20Result%20Structure%20%28by%20ref%29))
  ;[1 1 1] 攻击范围
  (Utilities|IsValid (Variables|Default|Get目标)
    (:Is%20Valid
      (Variables|Default|SetAttack true)
      (Variables|/Script/Engine.CharacterMovementComponent|SetMaxWalkSpeed (Variables|Character|GetCharacterMovement) 0.0)
      (CallFunction|LockRotationCF))))

(event OnComponentEndOverlap(攻击Sphere)
  (params (OverlappedComponent :type Primitive%20Component%20Object%20Reference) (OtherActor :type Actor%20Object%20Reference) (OtherComp :type Primitive%20Component%20Object%20Reference) (OtherBodyIndex :type Integer))
  (bind _目标_all (Variables|Default|Get目标_All))
  ;[1 1 1] 攻击范围内死亡
  (bind _as兵种_bp (Utilities|Casting|CastTo兵种_BP OtherActor))
  (Utilities|Array|RemoveItem (Variables|Default|Get目标_All) _as兵种_bp)
  (Variables|Default|SetAttack false)
  (if (> (Utilities|Array|Length _目标_all) 0)
    (Variables|Default|Set目标 (Utilities|Array|Get(acopy) _目标_all))
    (CallFunction|LockRotationCF)
    (else
      (Variables|Default|Set目标 0)))
  (Variables|/Script/Engine.CharacterMovementComponent|SetMaxWalkSpeed (Variables|Character|GetCharacterMovement) 6e+02))

(event Custom|InitInfo_CS
  (bind _returnvalue (Transformation|GetActorLocation))
  (bind _spline_bp (Variables|样条线|GetSpline_BP))
  (Utilities|FlowControl|Sequence
    (:then_0
      ;[1 1 1] 血条颜色设置
      (bind _ashp_umg (Utilities|Casting|CastToHP_UMG (UserInterface|GetUserWidgetObject (Variables|Default|GetWidget))))
      (bind _output_get (Variables|Default|SetHP%20UMG _ashp_umg))
      (Default|ChangeColorCF _output_get (Utilities|Select :Index "NewEnumerator0" :NewEnumerator0 "" :NewEnumerator5 "(R=1.000000,G=0.000000,B=0.000000,A=1.000000)" :NewEnumerator1 "(R=0.000000,G=0.000000,B=1.000000,A=1.000000)" :NewEnumerator3 "(R=0.000000,G=1.000000,B=0.000000,A=1.000000)"))
      (bind _output_get_2 (Variables|兵种属性|SetMax_HP 1e+02))
      (Variables|Default|SetCurrent_HP _output_get_2)
      (Development|SetHiddeninGame (Variables|Default|GetTextRender) true true))
    (:then_1
      ;[1 1 1] 初始位置设置
      (Variables|Default|SetStartPoint (Transformation|GetActorTransform))
      (Variables|Default|SetNewPoint _returnvalue)
      (Utilities|IsValid _spline_bp
        (:Is%20Valid
          (Variables|样条线|SetOffset (- _returnvalue (Transformation|GetActorLocation _spline_bp))))))))

(event Custom|CheckPoint_CS
  ;[1 1 1] AI
  (if (<= (Math|Vector|VectorLength (- (Transformation|GetActorLocation) (Variables|Default|GetNewPoint))) 2.5e+02)
    (CallFunction|UpdatePointCS)
    (goto _label Reset)
    (else
      (Utilities|FlowControl|DoOnce false :!label _label
        (:Completed
          (Utilities|IsValid (Variables|Default|Get目标)
            (:Is%20Not%20Valid
              (Variables|Default|SetAttack false)
              (Variables|/Script/Engine.CharacterMovementComponent|SetMaxWalkSpeed (Variables|Character|GetCharacterMovement) 6e+02))))))))

(event Custom|AImoveTo_CS
  (params (目标点 :type Transform) (移动结束后 :type Enum_移动类型%20Enum :default "NewEnumerator0") (Int :type Integer))
  (Variables|Default|Set展示 false)
  (bind _output_get (Variables|样条线|Set目标点 目标点))
  (Variables|兵种属性|SetEnum_移动类型 移动结束后)
  (AI|AIMoveTo self (.Location (Math|Transform|BreakTransform _output_get)) 0 5.0 false
    (:OnSuccess
      ;[1 1 1] 是否统一朝向
      (bind _新建轨道_0 (Timeline|时间轴_0 PlayFromStart)
        (:Update
          (Transformation|SetActorRotation (Math|Rotator|Lerp(Rotator) (Transformation|GetActorRotation self) (.Rotation (Math|Transform|BreakTransform _output_get)) _新建轨道_0)))
        (:Finished
          (CallFunction|举盾CS Int))))))

(event Custom|自定义事件_0
  (params (Self_ :type 兵种%20BP%20Object%20Reference))
  ;[1 1 1] 追击范围
  (Utilities|Array|RemoveItem (Variables|Default|Get目标_All) Self_))

(event Custom|SplineMove_CS
  ;[1 1 1] 沿样条线移动
  (Utilities|IsValid (Variables|样条线|GetSpline_BP)
    (:Is%20Valid
      (Variables|Default|Set展示 true)
      (Components|Timeline|SetPlayRate (Variables|Default|Get时间轴_样条线) (Variables|样条线|Get样条线移动速率))
      (bind _新建轨道_0 (Timeline|时间轴_样条线 PlayFromStart)
        (:Update
          (Transformation|SetActorTransform (Math|Transform|MakeTransform (+ (.Location (Math|Transform|BreakTransform (Default|GetWorldPointCF (Variables|样条线|GetSpline_BP) _新建轨道_0))) (Variables|样条线|GetOffset)) (.Rotation (Math|Transform|BreakTransform (Default|GetWorldPointCF (Variables|样条线|GetSpline_BP) _新建轨道_0))) (.Scale (Math|Transform|BreakTransform (Default|GetWorldPointCF (Variables|样条线|GetSpline_BP) _新建轨道_0))))))
        (:Finished
          (CallFunction|CSIFMakeDamage 9.99e+03))))))

(event Custom|TargetMove_CS
  ;[1 0.03646 0.03646] 暂停样条线移动，移动到目标点
  (Audio|Components|Audio|Stop (Variables|Default|Get时间轴_样条线))
  (Variables|样条线|SetSpline上位置 (Transformation|GetActorTransform)))

(event Custom|Run_CS
  (bind _目标 (Variables|Default|Get目标))
  (bind _startpoint (Variables|Default|GetStartPoint))
  (bind _returnvalue (Transformation|GetActorLocation _目标))
  (bind _returnvalue_2 (- _returnvalue (.location _startpoint)))
  (bind _returnvalue_3 (Math|Vector|Normalize _returnvalue_2))
  (bind _returnvalue_4 (* _returnvalue_3 -1.5e+03))
  (bind _returnvalue_5 (+ _returnvalue_4 (.location _startpoint)))
  ;[1 1 1] 反方向逃离目标
  (Rendering|Debug|DrawDebugArrow _returnvalue_5 (.RandomLocation (AI|Navigation|GetRandomReachablePointinRadius _returnvalue_5 2.5e+02 0 0)) 1e+01 "(R=1.000000,G=0.000000,B=0.000000,A=1.000000)" 1e+01 1e+01)
  (AI|AIMoveTo self (Math|Random|RandomPointinBoundingBox _returnvalue_5 "250.000000,250.000000, 0") 0 5e+01 false))

(event Custom|Attach_CS
  (params (目标 :type Actor%20Object%20Reference))
  ;[1 1 1] 附加，本意用于被箭射中后绑定在骨骼上，一起运动
  (Transformation|AttachComponentToComponent 目标 (Variables|Character|GetMesh) "None" "KeepWorld" "KeepWorld" "KeepWorld" true))

(event Custom|ChangeRate_CS
  (params (Reset :type Boolean))
  (bind _时间轴_样条线 (Variables|Default|Get时间轴_样条线))
  ;[1 1 1] 改变速度
  (if Reset
    (Components|Timeline|SetPlayRate _时间轴_样条线 (Variables|样条线|Get样条线移动速率))
    (else
      (bind _rate (Timeline|时间轴_1 PlayFromStart)
        (:Update
          (Components|Timeline|SetPlayRate _时间轴_样条线 _rate))))))

(event Custom|举盾_CS
  (params (Int :type Integer)))

(event Custom|UpdatePoint_CS
  (bind _pathspline_bp (Variables|Default|GetPathSpline_BP))
  (bind _targetsplineall (Variables|/Game/15/BP/AImoveTo_Spline_BP.AImoveTo_Spline_BP_C|GetTargetSplineAll _pathspline_bp))
  ;[1 1 1] AI
  (Utilities|FlowControl|Delay 0.0)
  (Development|PrintString "Hello++=UpdatePoint" true true "(R=0.000000,G=0.660000,B=1.000000,A=1.000000)" 5.0)
  (if (Variables|Default|GetRandom)
    (bind _output_get (Variables|Default|SetNewPoint (.RandomLocation (AI|Navigation|GetRandomReachablePointinRadius (Class|NavigationSystemV1|GetNavigationSystem) (Variables|Default|GetNewPoint) 5e+02 0 "/Game/15/AI/CS_NavFilter.CS_NavFilter_C")) :!label _label))
    (Rendering|Debug|DrawDebugSphere _output_get 15.0 12 "(R=1.000000,G=0.000000,B=0.000000,A=1.000000)" 1.0 3.0)
    (Utilities|FlowControl|DoOnce false
      (:Completed
        (Variables|/Script/Engine.CharacterMovementComponent|SetMaxWalkSpeed (Variables|Character|GetCharacterMovement) 4e+02)))
    (else
      (Utilities|IsValid _pathspline_bp
        (:Is%20Valid
          (bind _output_get_2 (Variables|Default|SetIndex (+ (Variables|Default|GetIndex) 1)))
          (if (>= _output_get_2 (Utilities|Array|Length _targetsplineall))
            (goto _label)
            (else
              (Variables|Default|SetNewPoint (.Location (Math|Transform|BreakTransform (Default|GetWorldPointCF (Utilities|Array|Get(acopy) _targetsplineall (Variables|Default|GetIndex)) (Variables|Default|GetDistance))))))))))))

(event EventBeginPlay
  (Utilities|FlowControl|Sequence
    (:then_0
      (CallFunction|InitInfoCS))
    (:then_1
      (switch Utilities|FlowControl|Switch|SwitchonEnum_移动类型 (Variables|兵种属性|GetEnum_移动类型)
        (:NewEnumerator0
          (CallFunction|ShowAnimCF (Variables|兵种属性|GetEnum_兵种状态%28展示%29)))
        (:NewEnumerator7
          (CallFunction|SplineMoveCS))
        (:NewEnumerator5
          (Variables|Default|SetRandom false))
        (:NewEnumerator1
          (Variables|Default|SetRandom true))))
    (:then_2
      (Utilities|FlowControl|Delay 2.0))))

(event EventCSIFMakeDamage
  (params (Damage :type Float%20%28single-precision%29))
  ;[1 1 1] 伤害判定，死亡，销毁
  (bind _die (CallFunction|DamageCF Damage))
  (if _die
    (Utilities|FlowControl|Sequence
      (:then_0
        (Variables|Default|Set展示 false)
        (Audio|Components|Audio|Stop (Variables|Default|Get时间轴_样条线))
        (Class|NavMovementComponent|StopActiveMovement (Variables|Character|GetCharacterMovement))
        (Collision|SetActorEnableCollision false))
      (:then_1
        (Variables|Default|SetDie true)
        (Utilities|FlowControl|Delay (Math|Random|RandomFloatinRange 1.0 2.0))
        (Actor|DestroyActor)))))

(event EventTick
  (params (DeltaSeconds :type Float%20%28single-precision%29))
  ;[1 1 1] 血条朝向，攻击手目标朝向
  (Utilities|FlowControl|Delay 0.1)
  (CallFunction|UpdateHPRotationCF))

(event EventCSIFAttack
  (bind _arrow1 (Variables|Default|GetArrow1))
  (bind _returnvalue (Transformation|GetWorldTransform _arrow1))
  (bind (_location _rotation _scale) (Math|Transform|BreakTransform _returnvalue))
  ;[1 1 1] 攻击
  (Utilities|FlowControl|Sequence
    (:then_0
      (CallFunction|LockRotationCF))
    (:then_1
      (Utilities|IsValid (Variables|Default|Get目标)
        (:Is%20Valid
          (for _index (range 0 5)
            (Variables|弓箭手瞄准|SetAimBox%20Extent (Math|Vector|MakeVector (Math|Float|MapRangeClamped (Math|Float|MapRangeClamped (Math|Vector|VectorLength (- (Transformation|GetActorLocation self) (Math|Random|RandomPointinBoundingBox (+ (Transformation|GetActorLocation (Variables|Default|Get目标)) (Math|Vector|MakeVector 0.0 0.0 (/ (Variables|/Script/Engine.CapsuleComponent|GetCapsuleHalfHeight (Variables|Collision|GetCapsuleComponent)) 2.0))) (Variables|弓箭手瞄准|GetAimBox%20Extent)))) 0.0 1e+03 0.1 0.3) 0.1 0.3 5e+01 2e+02) (Math|Float|MapRangeClamped (Math|Float|MapRangeClamped (Math|Vector|VectorLength (- (Transformation|GetActorLocation self) (Math|Random|RandomPointinBoundingBox (+ (Transformation|GetActorLocation (Variables|Default|Get目标)) (Math|Vector|MakeVector 0.0 0.0 (/ (Variables|/Script/Engine.CapsuleComponent|GetCapsuleHalfHeight (Variables|Collision|GetCapsuleComponent)) 2.0))) (Variables|弓箭手瞄准|GetAimBox%20Extent)))) 0.0 1e+03 0.1 0.3) 0.1 0.3 5e+01 2e+02) 1e+01))
            (Game|SpawnActorfromClass "/Game/帝国_农民/兵种人物动作/弩射手/箭_BP.箭_BP_C" (Math|Transform|MakeTransform _location "0, 0, 0" _scale) "Undefined" 0 (Variables|兵种属性|GetEnum_阵营) _location -9.8e+02 (Math|Random|RandomPointinBoundingBox (+ (Transformation|GetActorLocation (Variables|Default|Get目标)) (Math|Vector|MakeVector 0.0 0.0 (/ (Variables|/Script/Engine.CapsuleComponent|GetCapsuleHalfHeight (Variables|Collision|GetCapsuleComponent)) 2.0))) (Variables|弓箭手瞄准|GetAimBox%20Extent)) 0.5 self) ; 111--980\n0.3--0
          ))))))

(event EventCSIFFly
  (params (Point :type Vector :default "0, 0, 0") (Speed :type Vector :default "0, 0, 0"))
  (bind _returnvalue (Transformation|GetActorLocation))
  (bind _mesh (Variables|Character|GetMesh))
  (bind _returnvalue_2 (- _returnvalue Point))
  (bind _returnvalue_3 (Math|Vector|Normalize _returnvalue_2))
  (bind _returnvalue_4 (* _returnvalue_3 Speed))
  ;[1 1 1] 击飞
  (if (not (Variables|Default|GetDie))
    (Variables|Default|SetDie true)
    (Audio|Components|Audio|Stop (Variables|Default|Get时间轴_样条线))
    (Components|Movement|StopMovementImmediately (Variables|Character|GetCharacterMovement))
    (Character|LaunchCharacter (Math|Vector|MakeVector (.x _returnvalue_4) (.y _returnvalue_4) (.Z (Math|Vector|BreakVector Speed))) true true) ; 1000
    (Utilities|FlowControl|Delay 0.3)
    (Class|SkeletalMeshComponent|SetAllBodiesSimulatePhysics _mesh true)
    (Class|SkeletalMeshComponent|SetAllBodiesPhysicsBlendWeight _mesh 1.0 true)
    (Collision|SetCollisionEnabled _mesh "QueryAndPhysics")
    (Collision|SetCollisionEnabled (Variables|Collision|GetCapsuleComponent) "NoCollision")
    (Utilities|FlowControl|Delay (Math|Random|RandomFloatinRange 3.0 5.0))
    (Actor|DestroyActor)))

(event EventEndPlay
  (params (EndPlayReason :type EEndPlayReason%20Enum :default "Destroyed"))
  (Default|CallDestroyDis self))

(fn ConstructionScript)

(fn DamageCF
  (params (Damage :type Float%20%28single-precision%29))
  (bind _output_get (Variables|Default|SetCurrent_HP (- (Variables|Default|GetCurrent_HP) Damage)))
  (Default|UpdateHPCS (Variables|Default|GetHP%20UMG) (/ _output_get (Variables|兵种属性|GetMax_HP)))
  (return (<= _output_get 0.01)))

(fn UpdateHPRotationCF
  (bind _returnvalue (Game|GetPlayerCameraManager 0))
  (bind _widget (Variables|Default|GetWidget))
  (bind _returnvalue_2 (Transformation|GetWorldLocation _widget))
  (bind _returnvalue_3 (Transformation|GetActorLocation _returnvalue))
  (bind _returnvalue_4 (Math|Vector|MakeVector (.x _returnvalue_3) (.y _returnvalue_3) (.z _returnvalue_3)))
  (bind _returnvalue_5 (Math|Rotator|FindLookatRotation _returnvalue_2 _returnvalue_4))
  (Utilities|IsValid _widget
    (:Is%20Valid
      (Transformation|SetWorldRotation _widget (Math|Rotator|MakeRotator 0.0 (.pitch _returnvalue_5) (.yaw _returnvalue_5)) false false))))

(fn ShowAnimCF
  (params (Selection :type Enum_兵种状态%20Enum :default "NewEnumerator6"))
  (Variables|Default|Set展示 false)
  (Variables|Default|SetAttack false)
  (switch Utilities|FlowControl|Switch|SwitchonEnum_兵种状态 Selection
    (:NewEnumerator7
      (Variables|Default|Set展示 true))
    (:NewEnumerator5
      (Variables|Default|SetAttack true))))

(fn LockRotationCF
  (bind _returnvalue (Transformation|GetActorRotation))
  (bind _self self)
  (bind _aimbox_extent (Variables|弓箭手瞄准|GetAimBox%20Extent))
  (bind _目标 (Variables|Default|Get目标))
  (bind _returnvalue_2 (Transformation|GetActorLocation _self))
  (bind _returnvalue_3 (Transformation|GetActorLocation _目标))
  (bind _returnvalue_4 (Math|Random|RandomPointinBoundingBox _returnvalue_3 _aimbox_extent))
  (bind _returnvalue_5 (Math|Rotator|FindLookatRotation _returnvalue_2 _returnvalue_4))
  (bind (_roll _pitch _yaw) (Math|Rotator|BreakRotator _returnvalue_5))
  (Utilities|IsValid (Variables|Default|Get目标)
    (:Is%20Valid
      (if (not (Math|Vector|Equal(Vector) _returnvalue_3 (Variables|弓箭手瞄准|GetAimPoint) 1.0))
        (Variables|弓箭手瞄准|SetAimPoint _returnvalue_3)
        (Transformation|SetActorRotation (Math|Rotator|MakeRotator 0.0 0.0 (.Yaw (Math|Rotator|BreakRotator _returnvalue_5))))
        (Variables|弓箭手瞄准|SetAimRotation (Math|Rotator|MakeRotator (- (- (.pitch _returnvalue) _pitch) (Variables|弓箭手瞄准|GetPitchOffset)) (- _roll (.roll _returnvalue)) (- (- _yaw (.yaw _returnvalue)) (Variables|弓箭手瞄准|GetYawOffset))))))))

(fn InitInfoCF
  (params (Enum_阵营 :type Enum_阵营%20Enum :default "NewEnumerator0") (Enum_兵种状态%28展示%29 :type Enum_兵种状态%20Enum :default "NewEnumerator6") (Value :type Integer%20%28by%20ref%29))
  (Variables|兵种属性|SetEnum_阵营 Enum_阵营)
  (Variables|兵种属性|SetEnum_兵种状态%28展示%29 Enum_兵种状态%28展示%29)
  (Rendering|Components|TextRender|SetText (Variables|Default|GetTextRender) (Utilities|Text|ToText(Integer) Value)))

(fn CSIFGet阵营
  (return (Variables|兵种属性|GetEnum_阵营)))