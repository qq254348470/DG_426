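; 罗马盾兵_BP is the Blueprint for a Roman shield soldier unit.
; Show_CS sets the visibility of its Guangdun (light shield) component, while AttackCS is an empty event.
; BeginPlay and Tick are disabled parent-call stubs, overlap is empty, and the construction script only calls the parent.
; Unconnected leftovers hold a SetActive call and a faction check that would send a fly message to actors of another faction.
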(event Custom|Show_CS
  (params (bNewActive :type Boolean))
  (Rendering|SetVisibility (Variables|Default|Getguangdun) bNewActive false))

(event EventBeginPlay
  (|CallParentFunction) ; 此节点被禁用，将不会被调用。\n从引脚连出引线来编译功能。
)

(event Collision|EventActorBeginOverlap
  (params (OtherActor :type Actor%20Object%20Reference)))

(event EventTick
  (params (DeltaSeconds :type Float%20%28single-precision%29))
  (|CallParentFunction DeltaSeconds) ; 此节点被禁用，将不会被调用。\n从引脚连出引线来编译功能。
)

(event EventAttackCS)

(fn ConstructionScript
  (|CallParentFunction))