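; Test AI character that patrols around its spawn point, chases and attacks a 兵种_BP target, and returns when that target leaves the leash range.
; It takes its target from a delayed actor search or sphere overlap.
; Distance-check functions set the state and walk speed, and supply move points and targets to callers.
; Attacks play a crossbow montage alongside a looping re-check timer, then broadcast completion after a cooldown; perception handlers are empty.
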(event OnComponentBeginOverlap(Sphere)
  (params (OverlappedComponent :type Primitive%20Component%20Object%20Reference) (OtherActor :type Actor%20Object%20Reference) (OtherComp :type Primitive%20Component%20Object%20Reference) (OtherBodyIndex :type Integer) (bFromSweep :type Boolean) (SweepResult :type Hit%20Result%20Structure%20%28by%20ref%29))
  (bind _as兵种_bp (Utilities|Casting|CastTo兵种_BP OtherActor))
  (Utilities|IsValid (Variables|Default|GetTarget)
    (:Is%20Not%20Valid
      (Variables|Default|SetTarget _as兵种_bp))))

(event OnComponentEndOverlap(Sphere)
  (params (OverlappedComponent :type Primitive%20Component%20Object%20Reference) (OtherActor :type Actor%20Object%20Reference) (OtherComp :type Primitive%20Component%20Object%20Reference) (OtherBodyIndex :type Integer))
  (if (== OtherActor (Variables|Default|GetTarget))
    (CallFunction|UpdateTargetCF)))

(event OnPerceptionUpdated(AIPerception)
  (params (UpdatedActors :type Array%20of%20Actor%20Object%20References)))

(event OnTargetPerceptionUpdated(AIPerception)
  (params (Actor :type Actor%20Object%20Reference) (Stimulus :type AI%20Stimulus%20Structure)))

(event OnTargetPerceptionInfoUpdated(AIPerception)
  (params (UpdateInfo :type Actor%20Perception%20Update%20Info%20Structure%20%28by%20ref%29)))

(event Custom|StartAttack_CF
  (params (Attack :type Boolean))
  (if (Math|Boolean|NotEqual(Boolean) Attack (Variables|Default|GetAttack))
    (Variables|Default|SetAttack Attack)))

(event Custom|StartAttack_CS
  (Variables|/Script/Engine.CharacterMovementComponent|SetMaxWalkSpeed (Variables|Character|GetCharacterMovement) 0.0)
  (Animation|Montage|PlayMontage (Variables|Character|GetMesh) "/Game/帝国_农民/兵种人物动作/弩射手/5弩射手_Montage.5弩射手_Montage"
    (:then
      (if (Utilities|Time|IsValidTimerHandle (Variables|Default|GetTimer))
        (Utilities|Time|UnpauseTimerbyHandle (Variables|Default|GetTimer))
        (else
          (bind _returnvalue (Utilities|Time|SetTimerbyFunctionName self "UpdateTarget_CF" 0.1 true))
          (Variables|Default|SetTimer _returnvalue))))
    (:OnCompleted
      (Utilities|FlowControl|Sequence
        (:then_0
          (Utilities|FlowControl|Delay 1e+01)
          (Variables|/Script/Engine.CharacterMovementComponent|SetMaxWalkSpeed (Variables|Character|GetCharacterMovement) 6e+02)
          (Utilities|Time|PauseTimerbyHandle (Variables|Default|GetTimer))
          (Default|CallAttackEndEventDis))))))

(event EventBeginPlay
  (Variables|Default|SetStartPoint (Transformation|GetActorLocation))
  (Utilities|FlowControl|Delay 2.0)
  (bind _outactors (Actor|GetAllActorsOfClass "/Game/帝国_农民/兵种人物动作/弩射手/兵种_BP.兵种_BP_C"))
  (Variables|Default|SetTarget (Utilities|Array|Get(acopy) _outactors)))

(fn ConstructionScript)

(fn GetPointCF
  (switch Utilities|FlowControl|Switch|SwitchonEnum_StateAI (Variables|Default|GetEnum_StateAI)
    (:NewEnumerator1
      (bind _output_get (Variables|Default|SetRandom%20Location (.RandomLocation (Class|NavigationSystemV1|GetRandomPointinNavigableRadius (Variables|Default|GetStartPoint) (Variables|Default|Get巡逻范围) 0 0))))
      (Rendering|Debug|DrawDebugPoint _output_get 5.0 "(R=1.000000,G=0.000000,B=0.000000,A=1.000000)" 5.0)
      (return _output_get))
    (:NewEnumerator2
      (return (Transformation|GetActorLocation (Variables|Default|GetTarget))))
    (:NewEnumerator4
      (return (Variables|Default|GetStartPoint)))))

(fn GetTargetCF
  (CallFunction|StartAttackCF false)
  (Utilities|IsValid (Variables|Default|GetTarget)
    (:Is%20Valid
      (if (> (Math|Vector|VectorLength (- (Transformation|GetActorLocation (Variables|Default|GetTarget)) (Variables|Default|GetStartPoint))) (Variables|Default|Get返回范围))
        (Variables|/Script/Engine.CharacterMovementComponent|SetMaxWalkSpeed (Variables|Character|GetCharacterMovement) 6e+02)
        (Variables|Default|SetEnum_StateAI "NewEnumerator4")
        (Variables|Default|SetTarget 0)
        (return false 0 (Variables|Default|GetEnum_StateAI))
        (elif (< (Transformation|GetDistanceTo (Variables|Default|GetTarget) self) (Variables|Default|Get攻击范围))
          (Variables|Default|SetEnum_StateAI "NewEnumerator3")
          (CallFunction|StartAttackCF true)
          (return true (Variables|Default|GetTarget) (Variables|Default|GetEnum_StateAI))
          (elif (< (Transformation|GetDistanceTo (Variables|Default|GetTarget) self) (Variables|Default|Get追击范围))
            (Variables|/Script/Engine.CharacterMovementComponent|SetMaxWalkSpeed (Variables|Character|GetCharacterMovement) 1e+03)
            (Variables|Default|SetEnum_StateAI "NewEnumerator2")
            (return true (Variables|Default|GetTarget) (Variables|Default|GetEnum_StateAI))))))
    (:Is%20Not%20Valid
      (return false 0 (Variables|Default|GetEnum_StateAI)))))

(fn ChangeStateCF
  (params (Enum_StateAI :type Enum_StateAI%20Enum :default "NewEnumerator0"))
  (Variables|Default|SetEnum_StateAI Enum_StateAI))

(fn UpdateTargetCF
  (Utilities|IsValid (Variables|Default|GetTarget)
    (:Is%20Valid
      (if (> (Math|Vector|VectorLength (- (Transformation|GetActorLocation (Variables|Default|GetTarget)) (Variables|Default|GetStartPoint))) (Variables|Default|Get返回范围))
        (Variables|/Script/Engine.CharacterMovementComponent|SetMaxWalkSpeed (Variables|Character|GetCharacterMovement) 6e+02)
        (Variables|Default|SetEnum_StateAI "NewEnumerator4")
        (Variables|Default|SetTarget 0)
        (elif (< (Transformation|GetDistanceTo (Variables|Default|GetTarget) self) (Variables|Default|Get攻击范围))
          (Variables|Default|SetEnum_StateAI "NewEnumerator3")
          (Variables|/Script/Engine.CharacterMovementComponent|SetMaxWalkSpeed (Variables|Character|GetCharacterMovement) 0.0)
          (elif (< (Transformation|GetDistanceTo (Variables|Default|GetTarget) self) (Variables|Default|Get追击范围))
            (Variables|Default|SetEnum_StateAI "NewEnumerator2")
            (Variables|/Script/Engine.CharacterMovementComponent|SetMaxWalkSpeed (Variables|Character|GetCharacterMovement) 1e+03)))))))

(fn CSIFGet阵营
  (return "NewEnumerator0"))