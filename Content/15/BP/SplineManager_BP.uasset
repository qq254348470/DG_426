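; SplineManager_BP is a manager actor that lays out a set of Spline_BP paths and serves points sampled from them.
; Its construction script spawns a child actor at each SplineStart position with a fixed offset and rotation, caches it in AsSplineBP, and adds a text label showing its index.
; GetTargetPointsCF forwards a point request to the spline at the given index and returns the result.
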(event EventBeginPlay)

(event Collision|EventActorBeginOverlap
  (params (OtherActor :type Actor%20Object%20Reference)))

(event EventTick
  (params (DeltaSeconds :type Float%20%28single-precision%29)))

(fn ConstructionScript
  (Utilities|Array|Clear (Variables|Default|GetAs%20Spline%20BP))
  (for (_array_element _array_index) (Variables|Default|GetSplineStart)
    (bind _returnvalue (AddComponent|AddChildActorComponent false (Math|Transform|MakeTransform (+ _array_element "0.000000,100.000000, 0") "0,90.000000, 0" "1,1,1")))
    (bind _asaspline_bp (Utilities|Casting|CastToASpline_BP (Variables|/Script/Engine.ChildActorComponent|GetChildActor _returnvalue)))
    (Utilities|Array|Add (Variables|Default|GetAs%20Spline%20BP) _asaspline_bp)
    (bind _returnvalue_2 (AddComponent|AddTextRenderComponent false (Math|Transform|MakeTransform (+ _array_element "0, 0,50.000000") "0,90.000000, 0" "1,1,1")))
    (Rendering|Components|TextRender|SetText _returnvalue_2 (Utilities|Text|ToText(Integer) _array_index))))

(fn GetTargetPointsCF
  (params (InputPin :type Integer) (Num :type Integer))
  (bind _output_get (Variables|Default|SetPoints (Default|GetTargetDistancePointsCF (Utilities|Array|Get(acopy) (Variables|Default|GetAs%20Spline%20BP) InputPin) Num)))
  (return _output_get))