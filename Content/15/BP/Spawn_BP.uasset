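; Spawner actor that places a batch of AI units inside a box, passing each its faction, movement type, spline references and distance.
; When CanSpawn is set, BeginPlay starts a delayed one-shot timer that spawns the first SpawnClass entry and records units in AllAI.
; RandomSpawn picks grid-snapped random points or rotated rows evenly spread across the box width.
; Construction moves SplineBP onto the spawner; class cycling is left unwired.
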(event Custom|自定义事件_0
  (bind _spawnclass (Variables|Default|GetSpawnClass))
  (Variables|Default|SetCurrentClass (Utilities|Array|Get(acopy) _spawnclass (Math|Integer|Clamp(Integer) (Variables|Default|GetClassIndex) 0 (Utilities|Array|LastIndex _spawnclass))))
  (Math|Integer|IncrementInt (Variables|Default|GetClassIndex)))

(event Custom|Spawn
  (for _index (range 0 (Variables|Default|GetLast%20Index))
    (Variables|Default|SetDistance (Math|Float|%(Float) (* _index 0.1) 1.0))
    (bind _returnvalue (Game|SpawnActorfromClass (Variables|Default|GetCurrentClass) (Math|Transform|MakeTransform (Math|Vector|SelectVector (CallFunction|BoxRandomCF) (CallFunction|BoxLerpPointCF) (Variables|Default|GetRandomSpawn)) "0, 0, 0" "1,1,1") "AdjustIfPossibleButDontSpawnIfColliding" 0 (Variables|Default|GetEnum%20阵营) "NewEnumerator6" (Variables|Default|GetEnum_移动类型) (Variables|Default|GetSpline_BP) (Variables|Default|GetDistance) (Variables|Default|GetPathSpline_BP) 0))
    (Utilities|Array|Add (Variables|Default|GetAll_AI) _returnvalue)))

(event EventBeginPlay
  (if (Variables|Default|GetCanSpawn)
    (Utilities|FlowControl|Delay (Variables|Default|Get延迟))
    (bind _returnvalue (Utilities|Time|SetTimerbyEvent (delegate Custom|Spawn) 2.0)) ; 0.05---0.2
    (Variables|Default|SetTimer _returnvalue)
    (Utilities|FlowControl|Sequence
      (:then_0)
      (:then_1
        (Variables|Default|SetCurrentClass (Utilities|Array|Get(acopy) (Variables|Default|GetSpawnClass)))))))

(fn ConstructionScript
  (Transformation|SetActorLocation (Variables|Default|GetSpline_BP) (Transformation|GetActorLocation) false false))

(fn BoxRandomCF
  (bind _returnvalue (Transformation|GetActorLocation))
  (bind _box (Variables|Default|GetBox))
  (bind _returnvalue_2 (Components|Box|GetScaledBoxExtent _box))
  (bind (_x _y _z) (Math|Vector|BreakVector _returnvalue))
  (return (Math|Vector|MakeVector (+ _x (* (.ReturnValue (Math|Float|Division(WholeandRemainder) (Math|Random|RandomFloatinRange (* (.x _returnvalue_2) -1.0) (.x _returnvalue_2)) 5e+02)) 5e+02)) (+ _y (* (.ReturnValue (Math|Float|Division(WholeandRemainder) (Math|Random|RandomFloatinRange (* (.y _returnvalue_2) -1.0) (.y _returnvalue_2)) 5e+02)) 5e+02)) (+ _z (.Z (Math|Vector|BreakVector (Components|Box|GetScaledBoxExtent (Variables|Default|GetBox))))))))

(fn BoxLerpPointCF
  (bind _box (Variables|Default|GetBox))
  (bind _returnvalue (Components|Box|GetScaledBoxExtent _box))
  (return (+ (Math|Vector|RotateVector (Math|Vector|MakeVector (* (.ReturnValue (Math|Float|Division(WholeandRemainder) (Math|Random|RandomFloatinRange (* (.x _returnvalue) -1.0) (.x _returnvalue)) 1e+01)) 1e+01) (Math|Float|Lerp (* (.y _returnvalue) -1.0) (.y _returnvalue) (Variables|Default|GetDistance)) (.Z (Math|Vector|BreakVector (Components|Box|GetScaledBoxExtent (Variables|Default|GetBox))))) (Transformation|GetActorRotation)) (Transformation|GetActorLocation))))