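; Spline actor that builds a navigation line for AI behavior trees.
; Its construction script adds a child actor at each spline point's world transform, collects those cast to ASpline_BP in TargetSplineAll and passes each the point's scale.
; Helper functions return world transforms or locations from a fraction of spline length.
; GetRateCF dots against a zero vector, so its rate ignores the spline.
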(event Collision|EventActorBeginOverlap
  (params (OtherActor :type Actor%20Object%20Reference)))

(event EventTick
  (params (DeltaSeconds :type Float%20%28single-precision%29)))

(fn ConstructionScript
  (Utilities|Array|Clear (Variables|Default|GetTargetSplineAll))
  (Utilities|FlowControl|Sequence
    (:then_1
      (for _index (range 0 (- (Spline|GetNumberOfSplinePoints (Variables|Default|GetSpline)) 1))
        (bind _returnvalue (AddComponent|AddChildActorComponent true (Math|Transform|MakeTransform (.Return%20Value%20Location (CallFunction|GetPointLocationCF _index)) (.Return%20Value%20Rotation (CallFunction|GetPointLocationCF _index)) "1,1,1")))
        (bind _asaspline_bp (Utilities|Casting|CastToASpline_BP (Variables|/Script/Engine.ChildActorComponent|GetChildActor _returnvalue)))
        (Utilities|Array|Add (Variables|Default|GetTargetSplineAll) _asaspline_bp)
        (Default|UpdatePointCF _asaspline_bp (.Return%20Value%20Scale (CallFunction|GetPointLocationCF _index)))))))

(fn WorldCS
  (params (A :type Float%20%28single-precision%29))
  (bind _spline (Variables|Default|GetSpline))
  (return (Spline|GetTransformatDistanceAlongSpline _spline (* A (Spline|GetSplineLength _spline)) "World" false)))

(fn GetRateCF
  (params (A :type Float%20%28single-precision%29))
  (bind _spline (Variables|Default|GetSpline))
  (bind _returnvalue (Spline|GetSplineLength _spline))
  (bind _returnvalue_2 (* A _returnvalue))
  (bind _returnvalue_3 (- _returnvalue_2 1e+01))
  (bind _returnvalue_4 (Spline|GetLocationatDistanceAlongSpline _spline _returnvalue_3 "World"))
  (bind _returnvalue_5 (Math|Vector|DotProduct "0, 0, 0" _returnvalue_4))
  (bind _returnvalue_6 (Math|Float|NormalizetoRange _returnvalue_5 -3.0 1.0))
  (Development|PrintString (Utilities|String|ToString(Float) _returnvalue_6) true true "(R=1.000000,G=0.151505,B=0.000000,A=1.000000)")
  (return _returnvalue_6))

(fn GetDistancePointCF
  (params (Distance :type Float%20%28single-precision%29))
  (bind _spline (Variables|Default|GetSpline))
  (return (Spline|GetLocationatDistanceAlongSpline _spline (* Distance (Spline|GetSplineLength _spline)) "World")))

(fn GetPointLocationCF
  (params (PointIndex :type Integer))
  (bind _spline (Variables|Default|GetSpline))
  (bind _returnvalue (Spline|GetTransformatSplinePoint _spline PointIndex "World" true))
  (bind (_roll _pitch _yaw) (Math|Rotator|BreakRotator (.rotation _returnvalue)))
  (return (+ (.location _returnvalue) "0, 0, 0") (Math|Rotator|MakeRotator _roll _pitch (+ _yaw 0.0)) (.scale _returnvalue)))