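; Character Blueprint for a male farmer worker whose state sets both its animation and its held prop, covering jobs like mining, woodcutting, building, sowing and carrying.
; The state function loops the indexed animation at a given play rate on the farmer mesh, then selects the matching prop.
; A helper hides all props gathered from the mesh's children and shows the selected one.
; The current state is applied in both the construction script and BeginPlay.
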(event Collision|EventActorBeginOverlap
  (params (OtherActor :type Actor%20Object%20Reference)))

(event EventTick
  (params (DeltaSeconds :type Float%20%28single-precision%29)))

(event EventBeginPlay
  (CallFunction|改变状态CF (Variables|Default|Get农民状态) 1.0))

(fn ConstructionScript
  (Variables|Default|SetAll道具 (Components|GetChildrenComponents (Variables|Default|Get新男农民) false))
  (CallFunction|改变状态CF (Variables|Default|Get农民状态) 1.0))

(fn 隐藏道具CF
  (params (目标 :type Scene%20Component%20Object%20Reference))
  (for _array_element (Variables|Default|GetAll道具)
    (Rendering|SetVisibility _array_element false false))
  (Utilities|IsValid 目标
    (:Is%20Valid
      (Rendering|SetVisibility 目标 true false))))

(fn 改变状态CF
  (params (状态 :type 农民状态%20Enum :default "NewEnumerator0") (动画速率 :type Float%20%28single-precision%29))
  (bind _新男农民 (Variables|Default|Get新男农民))
  (Components|Animation|PlayAnimation _新男农民 (Utilities|Array|Get(acopy) (Variables|Default|Get动画) (Math|Conversions|ToInteger(Byte) 状态)) true)
  (Components|Timeline|SetPlayRate _新男农民 动画速率)
  (CallFunction|隐藏道具CF (Utilities|Select :Index 状态 :NewEnumerator0 (Variables|Default|Get旧铁凿_锄地) :NewEnumerator1 (Variables|Default|Get旧木头_搬运木头) :NewEnumerator2 (Variables|Default|Get旧篮子_采集野果) :NewEnumerator3 (Variables|Default|Get旧金矿_搬运金矿) :NewEnumerator4 (Variables|Default|Get旧斧头_伐木) :NewEnumerator5 (Variables|Default|Get旧锤子_建造) :NewEnumerator11 (Variables|Default|Get旧斧头_走) :NewEnumerator12 (Variables|Default|Get旧锄头_走) :NewEnumerator13 (Variables|Default|Get旧锤子_走) :NewEnumerator6 (Variables|Default|Get旧抗铁凿_走) :NewEnumerator7 (Variables|Default|Get旧铁凿_挖矿) :NewEnumerator8 (Variables|Default|Get旧簸箕_播种) :NewEnumerator9 (Variables|Default|Get旧簸箕_播种走) :NewEnumerator10 (Variables|Default|Get旧铁凿_锄地))))